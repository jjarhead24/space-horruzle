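; BP_Item_01 is a pickup item that a player can use to add to their inventory.
; The construction script looks up the row at index ID in Inventory_DT's row names and applies its mesh, name and value.
; BeginPlay caches the first-person character, and UseAction passes the ID to that character's AddToInventory, then destroys the item.
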(event EventBeginPlay
  (bind _asbp_first_person_character (Utilities|Casting|CastToBP_FirstPersonCharacter (Game|GetPlayerCharacter 0)))
  (Variables|Default|SetAs%20BP%20First%20Person%20Character _asbp_first_person_character))

(event Collision|EventActorBeginOverlap
  (params (OtherActor :type Actor%20Object%20Reference)))

(event EventTick
  (params (DeltaSeconds :type Float%20%28single-precision%29)))

(event EventUseAction
  (Default|AddtoInventory (Variables|Default|GetAs%20BP%20First%20Person%20Character) (Variables|Default|GetID))
  (Actor|DestroyActor))

(fn ConstructionScript
  (bind _outrownames (DataTable|GetDataTableRowNames "/Game/Inventory/Inventory_DT.Inventory_DT"))
  (bind _returnvalue (Utilities|GetDataTableRow "/Game/Inventory/Inventory_DT.Inventory_DT" (Utilities|Array|Get(acopy) _outrownames (Variables|Default|GetID)))
    (:then
      (Components|StaticMesh|SetStaticMesh (Variables|Default|GetStaticMesh) (.Mesh (Utilities|Struct|BreakInventory_Struc _returnvalue)))
      (Variables|Default|SetName (.Name (Utilities|Struct|BreakInventory_Struc _returnvalue)))
      (Variables|Default|SetValue (.Value (Utilities|Struct|BreakInventory_Struc _returnvalue))))))