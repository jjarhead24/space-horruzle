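; Cog puzzle Blueprint that unlocks a valve controlling steam in a linked pipe once the required number of cogs is fitted.
; UseAction either adjusts the cog count, marking the puzzle complete only on an exact match, or handles valve interaction.
; When complete, using the valve toggles the pipe's steam and plays the Turn timeline forward or in reverse, lerping the valve between start and end rotations.
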(event EventBeginPlay
  (Variables|Default|SetStartRotation (Variables|/Script/Engine.SceneComponent|GetRelativeRotation (Variables|Default|Getvalve)))
  (Variables|Default|SetEndRotation (Variables|Default|GetEndRotation)))

(event EventUseAction
  (params (Cog_added :type Boolean) (no_cog_change :type Boolean) (Valve_interact :type Boolean))
  (bind _pipe (Variables|Default|GetPipe))
  (if no_cog_change
    (if Valve_interact
      (if (Variables|Default|GetComplete)
        (if (Variables|/Game/BluePrints/Broke_pipe_BP.Broke_pipe_BP_C|Getcurrent%20steam _pipe)
          (Default|UpdateSteam _pipe false)
          (bind _valve_turn (Timeline|turn PlayFromStart)
            (:Update
              (Transformation|SetRelativeRotation (Variables|Default|Getvalve) (Math|Rotator|Lerp(Rotator) (Variables|Default|GetStartRotation) (Variables|Default|GetEndRotation) _valve_turn) false false))
            (:Finished
              (Development|PrintString (Utilities|String|ToString(Boolean) (Variables|/Game/BluePrints/Broke_pipe_BP.Broke_pipe_BP_C|Getcurrent%20steam (Variables|Default|GetPipe))))))
          (else
            (Default|UpdateSteam _pipe true)
            (Timeline|turn Reverse)))))
    (else
      (if Cog_added
        (Variables|Default|SetCog_on (+ (Variables|Default|GetCog_on) 1))
        (else
          (Variables|Default|SetCog_on (- (Variables|Default|GetCog_on) 1))))
      (if (== (Variables|Default|GetCog_on) (Variables|Default|GetCog_needed))
        (Variables|Default|SetComplete true)
        (Development|PrintString "done")
        (else
          (Variables|Default|SetComplete false))))))

(fn ConstructionScript)