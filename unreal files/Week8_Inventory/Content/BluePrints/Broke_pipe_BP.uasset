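; Broken pipe Blueprint that shows or hides a Niagara effect and reacts when something enters its trigger box.
; UpdateSteam sets the Steam flag and toggles the Niagara component's visibility to match.
; On box overlap, active steam prints a debug "ouchie" only for the first-person character, while inactive steam prints "whew" for any actor.
; No damage is applied.
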(event OnComponentBeginOverlap(Box)
  (params (OverlappedComponent :type Primitive%20Component%20Object%20Reference) (OtherActor :type Actor%20Object%20Reference) (OtherComp :type Primitive%20Component%20Object%20Reference) (OtherBodyIndex :type Integer) (bFromSweep :type Boolean) (SweepResult :type Hit%20Result%20Structure%20%28by%20ref%29))
  (if (Variables|Default|GetSteam)
    (Utilities|Casting|CastToBP_FirstPersonCharacter OtherActor)
    (Development|PrintString "ouchie")
    (else
      (Development|PrintString "whew"))))

(event EventBeginPlay)

(event Collision|EventActorBeginOverlap
  (params (OtherActor :type Actor%20Object%20Reference)))

(event EventTick
  (params (DeltaSeconds :type Float%20%28single-precision%29)))

(fn ConstructionScript)

(fn UpdateSteam
  (params (new_steam :type Boolean))
  (bind _niagara (Variables|Default|GetNiagara))
  (if new_steam
    (Rendering|SetVisibility _niagara true false)
    (Variables|Default|SetSteam true)
    (else
      (Rendering|SetVisibility _niagara false false)
      (Variables|Default|SetSteam false))))