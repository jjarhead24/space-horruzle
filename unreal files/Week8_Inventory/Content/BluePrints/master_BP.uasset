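; Base damageable actor with a chamfer-cube mesh and a floating label showing its name and health.
; The construction script sets the mesh and label, and Tick rotates the label to face the player camera.
; AnyDamage lowers clamped health and refreshes the label.
; At zero health the actor is flagged dead and its death event destroys it.
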(event Custom|Event%20Death
  (Actor|DestroyActor))

(event EventBeginPlay)

(event Collision|EventActorBeginOverlap
  (params (OtherActor :type Actor%20Object%20Reference)))

(event EventTick
  (params (DeltaSeconds :type Float%20%28single-precision%29))
  (Transformation|SetRelativeRotation (Variables|Default|Gettext) (Math|Rotator|FindLookatRotation (Transformation|GetActorLocation) (Transformation|GetActorLocation (Game|GetPlayerCameraManager 0))) false false))

(event Game|Damage|EventAnyDamage
  (params (Damage :type Float%20%28single-precision%29) (DamageType :type Damage%20Type%20Object%20Reference) (InstigatedBy :type Controller%20Object%20Reference) (DamageCauser :type Actor%20Object%20Reference))
  (CallFunction|UpdateHealth Damage)
  (CallFunction|UpdateText))

(fn ConstructionScript
  (Components|StaticMesh|SetStaticMesh (Variables|Default|Getmesh) "/Game/LevelPrototyping/Meshes/SM_ChamferCube.SM_ChamferCube")
  (CallFunction|UpdateText))

(fn UpdateText
  (if (not (Variables|Default|GetIsDead))
    (Rendering|Components|TextRender|SetText (Variables|Default|Gettext) (Utilities|Text|FormatText "{Name} {Health}" (Variables|Default|GetName) (Variables|Default|GetHealth)))))

(fn UpdateHealth
  (params (Damage :type Float%20%28double-precision%29))
  (bind _output_get (Variables|Default|SetHealth (Math|Float|Clamp(Float) (- (Variables|Default|GetHealth) Damage) 0.0 1e+02)))
  (if (== _output_get 0.0)
    (Variables|Default|SetIsDead true)
    (CallFunction|EventDeath)))