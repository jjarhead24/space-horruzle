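; Cog puzzle Blueprint that tracks how many cogs are in place and flags the puzzle as complete.
; Its UseAction event takes a CogAdded flag, raising or lowering the CogOn count accordingly.
; When the count equals CogNeeded it sets Complete and prints a debug message; otherwise it clears Complete, so removing a cog can undo completion.
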(event EventBeginPlay)

(event Collision|EventActorBeginOverlap
  (params (OtherActor :type Actor%20Object%20Reference)))

(event EventTick
  (params (DeltaSeconds :type Float%20%28single-precision%29)))

(event EventUseAction
  (params (Cog_added :type Boolean))
  (if Cog_added
    (Variables|Default|SetCog_on (+ (Variables|Default|GetCog_on) 1))
    (else
      (Variables|Default|SetCog_on (- (Variables|Default|GetCog_on) 1))))
  (if (== (Variables|Default|GetCog_on) (Variables|Default|GetCog_needed))
    (Variables|Default|SetComplete true)
    (Development|PrintString "done")
    (else
      (Variables|Default|SetComplete false))))

(fn ConstructionScript)