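; BP_Item_01 is a pickup item that adds itself to the first-person character's inventory.
; The construction script uses ID to index the Inventory_DT row names, setting mesh, material, Name and Value from that row.
; It also assigns a Niagara pickup effect and feeds it the Coggers static mesh.
; UseAction passes ID to the cached character's AddToInventory and destroys the actor only if that succeeds.
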(event EventBeginPlay
  (bind _asbp_first_person_character (Utilities|Casting|CastToBP_FirstPersonCharacter (Game|GetPlayerCharacter 0)))
  (Variables|Default|SetAs%20BP%20First%20Person%20Character _asbp_first_person_character))

(event Collision|EventActorBeginOverlap
  (params (OtherActor :type Actor%20Object%20Reference)))

(event EventTick
  (params (DeltaSeconds :type Float%20%28single-precision%29)))

(event EventUseAction
  (params (Cog_added :type Boolean))
  (bind _success (Default|AddtoInventory (Variables|Default|GetAs%20BP%20First%20Person%20Character) (Variables|Default|GetID)))
  (if _success
    (Actor|DestroyActor)))

(fn ConstructionScript
  (bind _niagara (Variables|Default|GetNiagara))
  (bind _outrownames (DataTable|GetDataTableRowNames "/Game/FirstPerson/Inventory/Inventory_DT.Inventory_DT"))
  (bind _returnvalue (Utilities|GetDataTableRow "/Game/FirstPerson/Inventory/Inventory_DT.Inventory_DT" (Utilities|Array|Get(acopy) _outrownames (Variables|Default|GetID)))
    (:then
      (Components|StaticMesh|SetStaticMesh (Variables|Default|GetStaticMesh) (.Mesh (Utilities|Struct|BreakInventory_Struc _returnvalue)))
      (Rendering|Material|SetMaterial (Variables|Default|GetStaticMesh) 0 (.Material (Utilities|Struct|BreakInventory_Struc _returnvalue)))
      (Variables|Default|SetName (.Name (Utilities|Struct|BreakInventory_Struc _returnvalue)))
      (Variables|Default|SetValue (.ID (Utilities|Struct|BreakInventory_Struc _returnvalue)))
      (Class|NiagaraComponent|SetAsset _niagara "/Game/FX/show_pickup_System.show_pickup_System" true)
      (Class|NiagaraComponent|SetVariableStaticMesh _niagara "StaticMesh" "/Game/Assets/Coggers.Coggers"))))